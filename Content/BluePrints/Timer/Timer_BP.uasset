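; Timer_BP is a short-lived visual timer actor that shows elapsed time through a material on TimerMesh.
; BeginPlay records the start time and destroys the actor after a delay of just over a second.
; Each Tick writes the elapsed seconds, scaled to a percentage, into the material's Percentage scalar parameter.
; The Construction Script sets the same parameter from the Percentage variable, giving the mesh its initial fill value.
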(event EventBeginPlay
  (Variables|Default|SetStart%20Time (Utilities|Time|GetTimeSeconds))
  (Utilities|FlowControl|Delay 1.1)
  (Actor|DestroyActor))

(event Collision|EventActorBeginOverlap
  (params (OtherActor :type Actor%20Object%20Reference)))

(event EventTick
  (params (DeltaSeconds :type Float%20%28single-precision%29))
  (Rendering|Material|SetScalarParameterValueonMaterials (Variables|Default|GetTimer_Mesh) "Percentage" (* 100 (- (Utilities|Time|GetTimeSeconds) (Variables|Default|GetStart%20Time)))))

(fn ConstructionScript
  (Rendering|Material|SetScalarParameterValueonMaterials (Variables|Default|GetTimer_Mesh) "Percentage" (Variables|Default|GetPercentage)))