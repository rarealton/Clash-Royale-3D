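; A one-second timer actor that shows elapsed time with a rotating hand and a material-driven timer mesh, then destroys itself.
; On BeginPlay it records the start time and plays a timeline that pitches the hand, destroying the actor when finished.
; Tick sets the mesh's Percentage material parameter to 100 times the elapsed seconds.
; The construction script applies the Percentage variable to the same parameter for the initial look.
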(event EventBeginPlay
  (Variables|Default|SetStart%20Time (Utilities|Time|GetTimeSeconds))
  (bind _rotation (Timeline|Hand_Rot PlayFromStart)
    (:Update
      (Transformation|SetRelativeRotation (Variables|Default|GetHand) (Math|Rotator|MakeRotator 0.0 _rotation 0.0) false false))
    (:Finished
      (Actor|DestroyActor))))

(event Collision|EventActorBeginOverlap
  (params (OtherActor :type Actor%20Object%20Reference)))

(event EventTick
  (params (DeltaSeconds :type Float%20%28single-precision%29))
  (Rendering|Material|SetScalarParameterValueonMaterials (Variables|Default|GetTimer_Mesh) "Percentage" (* 100 (- (Utilities|Time|GetTimeSeconds) (Variables|Default|GetStart%20Time)))))

(fn ConstructionScript
  (Rendering|Material|SetScalarParameterValueonMaterials (Variables|Default|GetTimer_Mesh) "Percentage" (Variables|Default|GetPercentage)))