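; ArenaTower is an arena tower actor with two banners that displays either blue or red team colors.
; The Construction Script reads the TeamBlue flag and sets a team material on one slot of the tower mesh and on both banners.
; The event graph holds only disabled stub events, so the Blueprint has no runtime logic of its own.
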(event EventBeginPlay)

(event Collision|EventActorBeginOverlap
  (params (OtherActor :type Actor%20Object%20Reference)))

(event EventTick
  (params (DeltaSeconds :type Float%20%28single-precision%29)))

(fn ConstructionScript
  (bind _arenatower (Variables|Default|GetArenaTower))
  (if (Variables|Default|GetTeamBlue?)
    (Rendering|Material|SetMaterial _arenatower 4 "/Game/Materials/Instances/Dark_Blue_Inst.Dark_Blue_Inst")
    (Rendering|Material|SetMaterial (Variables|Default|GetBanner) 0 "/Game/Materials/Instances/Banner_Blue.Banner_Blue")
    (else
      (Rendering|Material|SetMaterial _arenatower 4 "/Game/Materials/Instances/Dark_Red_Inst.Dark_Red_Inst")
      (Rendering|Material|SetMaterial (Variables|Default|GetBanner) 0 "/Game/Materials/Instances/Banner_Red.Banner_Red"))))