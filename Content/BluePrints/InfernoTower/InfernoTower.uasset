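; Inferno Tower actor that locks a particle beam onto the player while they are inside its Sight volume; no damage is applied here.
; Sight overlaps set a flag that Tick reads to aim and toggle the beam after a short initial delay.
; Two seconds into a lock, Tick boosts the tower material's distortion and pulse parameters, with no reset.
; TeamBlue picks material and health-bar color; Tick refreshes the health widget.
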(event OnComponentBeginOverlap(Sight)
  (params (OverlappedComponent :type Primitive%20Component%20Object%20Reference) (OtherActor :type Actor%20Object%20Reference) (OtherComp :type Primitive%20Component%20Object%20Reference) (OtherBodyIndex :type Integer) (bFromSweep :type Boolean) (SweepResult :type Hit%20Result%20Structure%20%28by%20ref%29))
  (Utilities|Casting|CastToFirstPersonCharacter OtherActor)
  (Variables|Default|SetHas%20Player%20in%20Sight true))

(event OnComponentEndOverlap(Sight)
  (params (OverlappedComponent :type Primitive%20Component%20Object%20Reference) (OtherActor :type Actor%20Object%20Reference) (OtherComp :type Primitive%20Component%20Object%20Reference) (OtherBodyIndex :type Integer))
  (Utilities|Casting|CastToFirstPersonCharacter OtherActor)
  (Variables|Default|SetHas%20Player%20in%20Sight false))

(event EventBeginPlay
  ;[1 1 1] Set Progress Bar Color
  (bind _asinferno_tower_health (Utilities|Casting|CastToInfernoTowerHealth (UserInterface|GetUserWidgetObject (Variables|Default|GethealthBar))))
  (if (Variables|Default|GetTeamBlue?)
    (Class|ProgressBar|SetFillColorandOpacity (Variables|/Game/BluePrints/InfernoTower/InfernoTowerHealth.InfernoTowerHealth_C|GetHealthBar _asinferno_tower_health) "(R=0.000000,G=0.056455,B=0.620000,A=1.000000)")
    (else
      (Class|ProgressBar|SetFillColorandOpacity (Variables|/Game/BluePrints/InfernoTower/InfernoTowerHealth.InfernoTowerHealth_C|GetHealthBar _asinferno_tower_health) "(R=0.565000,G=0.000000,B=0.000000,A=1.000000)"))))

(event EventTick
  (params (DeltaSeconds :type Float%20%28single-precision%29))
  (bind _returnvalue (Game|GetPlayerCharacter 0))
  (bind _returnvalue_2 (Game|GetPlayerCharacter 0))
  (bind _inferno_tower (Variables|Default|GetInferno_Tower))
  (bind _returnvalue_3 (Transformation|GetActorLocation _returnvalue_2))
  (bind _returnvalue_4 (Transformation|GetActorLocation _returnvalue))
  (bind _returnvalue_5 (+ _returnvalue_3 "0.000000,0.000000,30.000000"))
  (bind _returnvalue_6 (+ _returnvalue_4 "0.000000,0.000000,30.000000"))
  ;[1 1 1] Set Progress Bar Percent
  (bind _asinferno_tower_health (Utilities|Casting|CastToInfernoTowerHealth (UserInterface|GetUserWidgetObject (Variables|Default|GethealthBar)))
    (:then
      _)
    (:CastFailed
      _))
  (Variables|/Game/BluePrints/InfernoTower/InfernoTowerHealth.InfernoTowerHealth_C|SetHealth _asinferno_tower_health (Utilities|Text|ToText(Float) (Variables|Default|GetHealth) "HalfToEven"))
  (Progress|SetPercent (Variables|/Game/BluePrints/InfernoTower/InfernoTowerHealth.InfernoTowerHealth_C|GetHealthBar _asinferno_tower_health) (/ (Variables|Default|GetHealth) 1e+02))
  ;[1 1 1] Beam Logic
  (if (Variables|Default|GetHas%20Player%20in%20Sight)
    (if (Variables|Default|GetDoneDelay)
      _
      (else
        (Utilities|FlowControl|Delay 0.8)
        (Variables|Default|SetDoneDelay true)
        (Variables|Default|SetLock%20Begin%20Time (Utilities|Time|GetTimeSeconds))))
    (Class|ParticleSystemComponent|SetBeamTargetPoint (Variables|Default|GetInfernoBeam) 1 _returnvalue_5)
    (Effects|Components|ParticleSystem|SetVectorParameter (Variables|Default|GetInfernoBeam) "Attract Location" _returnvalue_5)
    (Rendering|SetVisibility (Variables|Default|GetInfernoBeam) true false)
    (if (not (<= (- (Utilities|Time|GetTimeSeconds) (Variables|Default|GetLock%20Begin%20Time)) 2.0))
      (Rendering|Material|SetScalarParameterValueonMaterials _inferno_tower "Distance Strength" 5e+02)
      (Rendering|Material|SetScalarParameterValueonMaterials _inferno_tower "Pulse Strength" 5e+02))
    (else
      (Variables|Default|SetDoneDelay false)
      (Rendering|SetVisibility (Variables|Default|GetInfernoBeam) false false)
      (if (not false)
        (Class|ParticleSystemComponent|SetBeamTargetPoint (Variables|Default|GetInfernoBeam) 1 _returnvalue_6)
        (Effects|Components|ParticleSystem|SetVectorParameter (Variables|Default|GetInfernoBeam) "Attract Location" _returnvalue_6)))))

(fn ConstructionScript
  (if (Variables|Default|GetTeamBlue?)
    (Rendering|Material|SetMaterial (Variables|Default|GetInferno_Tower) 4 "/Game/Materials/Instances/Dark_Blue_Inst.Dark_Blue_Inst")
    (else
      (Rendering|Material|SetMaterial (Variables|Default|GetInferno_Tower) 4 "/Game/Materials/Instances/Dark_Red_Inst.Dark_Red_Inst"))))