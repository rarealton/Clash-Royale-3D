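; Cinematic spotlight actor that pairs a SpotLight component with a mesh, Cylinder1, that has a tintable glow material.
; The construction script applies the exposed intensity and color variables to the light.
; It separately writes glow color and intensity into the cylinder's "Color" and "Intensity" material parameters, so the glow is set independently of the light.
; It has no runtime logic; the event graph holds only disabled placeholder events.
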(event EventBeginPlay)

(event Collision|EventActorBeginOverlap
  (params (OtherActor :type Actor%20Object%20Reference)))

(event EventTick
  (params (DeltaSeconds :type Float%20%28single-precision%29)))

(fn ConstructionScript
  (bind _glow_color (Variables|Default|GetGlow%20Color))
  (bind _spotlight (Variables|Default|GetSpotLight))
  (bind (_r _g _b) (Math|Color|BreakColor _glow_color))
  (Rendering|Components|Light|SetIntensity _spotlight (Variables|Default|GetIntensity))
  (Rendering|Components|Light|SetLightColor _spotlight (Variables|Default|GetLight%20Color) true)
  (Rendering|Material|SetVectorParameterValueonMaterials (Variables|Default|GetCylinder1) "Color" (Math|Vector|MakeVector _r _g _b))
  (Rendering|Material|SetScalarParameterValueonMaterials (Variables|Default|GetCylinder1) "Intensity" (Variables|Default|GetGlow%20Intensity)))