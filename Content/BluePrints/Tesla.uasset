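; Tesla tower that raises itself and aims a lightning beam at the player character when it enters the Sight volume.
; Chained Glow and Z_Height timelines open two mirrored door pivots and lift the coil, reversing Z_Height when the player leaves.
; After a brief delay, Tick tracks the player with the beam, toggling visibility on time parity to flicker.
; The construction script sets team color and optionally starts the coil raised.
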(event OnComponentBeginOverlap(Sight)
  (params (OverlappedComponent :type Primitive%20Component%20Object%20Reference) (OtherActor :type Actor%20Object%20Reference) (OtherComp :type Primitive%20Component%20Object%20Reference) (OtherBodyIndex :type Integer) (bFromSweep :type Boolean) (SweepResult :type Hit%20Result%20Structure%20%28by%20ref%29))
  (Utilities|Casting|CastToFirstPersonCharacter OtherActor)
  (Variables|Default|SetHas%20Player%20in%20Sight true)
  (bind _newtrack_0 (Timeline|Glow PlayFromStart)
    (:Update
      (bind (_direction _z_position _doors) (Timeline|Z_Height Play)
        (:Update
          (Transformation|SetRelativeRotation (Variables|Default|GetDoor_Pivot) (Math|Rotator|MakeRotator _doors 0.0 0.0) false false)
          (Transformation|SetRelativeRotation (Variables|Default|GetDoor_Pivot2) (* (Math|Rotator|MakeRotator _doors 0.0 0.0) -1) false false)
          (Transformation|SetRelativeLocation (Variables|Default|GetTesla) (Math|Vector|MakeVector 0.0 0.0 _z_position) false false))))))

(event OnComponentEndOverlap(Sight)
  (params (OverlappedComponent :type Primitive%20Component%20Object%20Reference) (OtherActor :type Actor%20Object%20Reference) (OtherComp :type Primitive%20Component%20Object%20Reference) (OtherBodyIndex :type Integer))
  (bind _output_get (Variables|Default|SetTargets OtherActor))
  (Utilities|Casting|CastToFirstPersonCharacter _output_get)
  (Variables|Default|SetHas%20Player%20in%20Sight false)
  (bind (_direction _z_position _doors) (Timeline|Z_Height Reverse)
    (:Update
      (Transformation|SetRelativeRotation (Variables|Default|GetDoor_Pivot) (Math|Rotator|MakeRotator _doors 0.0 0.0) false false)
      (Transformation|SetRelativeRotation (Variables|Default|GetDoor_Pivot2) (* (Math|Rotator|MakeRotator _doors 0.0 0.0) -1) false false)
      (Transformation|SetRelativeLocation (Variables|Default|GetTesla) (Math|Vector|MakeVector 0.0 0.0 _z_position) false false))))

(event Collision|EventActorBeginOverlap
  (params (OtherActor :type Actor%20Object%20Reference)))

(event EventTick
  (params (DeltaSeconds :type Float%20%28single-precision%29))
  (if (Variables|Default|GetHas%20Player%20in%20Sight)
    (if (Variables|Default|GetDoneDelay)
      _
      (else
        (Utilities|FlowControl|Delay 0.8)
        (Variables|Default|SetDoneDelay true)))
    (Class|ParticleSystemComponent|SetBeamTargetPoint (Variables|Default|GetLightning) 0 (Transformation|GetActorLocation (stale OnComponentEndOverlap(Sight) _output_get)))
    (if (== (Math|Integer|%(Integer) (Math|Float|Truncate (* 10 (Utilities|Time|GetTimeSeconds))) 2) 0)
      (Utilities|FlowControl|DoOnce false :!label _label
        (:Completed
          (bind _isa (Utilities|FlowControl|FlipFlop)
            (:A
              _)
            (:B
              _))
          (Rendering|SetVisibility (Variables|Default|GetLightning) _isa false)))
      (else
        (goto _label Reset)))
    (else
      (Variables|Default|SetDoneDelay false)
      (Rendering|SetVisibility (Variables|Default|GetLightning) false false)
      (if (not false)
        (Class|ParticleSystemComponent|SetBeamTargetPoint (Variables|Default|GetLightning) 0 (Transformation|GetActorLocation (stale OnComponentEndOverlap(Sight) _output_get)))))))

(event EventBeginPlay
  (Variables|Default|SetTargets (Game|GetPlayerCharacter 0)))

(fn ConstructionScript
  (bind _returnvalue (Math|Rotator|MakeRotator 5e+01 0.0 0.0))
  (bind _tesla (Variables|Default|GetTesla))
  (if (Variables|Default|GetTeamBlue?)
    (Rendering|Material|SetMaterial _tesla 1 "/Game/Materials/Instances/Dark_Blue_Inst.Dark_Blue_Inst")
    (else
      (Rendering|Material|SetMaterial _tesla 1 "/Game/Materials/Instances/Dark_Red_Inst.Dark_Red_Inst")))
  (if (Variables|Default|GetSetInitHeight?)
    (Transformation|AddLocalOffset (Variables|Default|GetTesla) "0, 0,840.000000" false false)
    (Transformation|SetRelativeRotation (Variables|Default|GetDoor_Pivot) _returnvalue false false)
    (Transformation|SetRelativeRotation (Variables|Default|GetDoor_Pivot2) (* _returnvalue -1) false false)))