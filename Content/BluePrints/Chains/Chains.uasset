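; Spline-driven chain actor that builds a chain of metal link meshes along an editable spline.
; The construction script divides the spline length by Spacing and adds a static mesh component at each step, shifted by ChainOffset.
; Each link follows the spline's rotation with an extra 90 degrees of roll per index, so neighbouring links interlock at right angles.
; The event graph holds no logic.
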(event EventBeginPlay)

(event Collision|EventActorBeginOverlap
  (params (OtherActor :type Actor%20Object%20Reference)))

(event EventTick
  (params (DeltaSeconds :type Float%20%28single-precision%29)))

(fn ConstructionScript
  (bind _spacing (Variables|Default|GetSpacing))
  (bind _spline (Variables|Default|GetSpline))
  (for _index (range 0 (.ReturnValue (Math|Float|Division(WholeandRemainder) (Spline|GetSplineLength (Variables|Default|GetSpline)) _spacing)))
    (bind _returnvalue (AddComponent|AddStaticMeshComponent false (Math|Transform|MakeTransform (+ (Spline|GetLocationatDistanceAlongSpline _spline (* _index _spacing) "Local") (Variables|Default|GetChain%20Offset)) (Math|Rotator|MakeRotator (+ (Math|Conversions|ToFloat(Integer) (* _index 90)) (.Roll (Math|Rotator|BreakRotator (Spline|GetRotationatDistanceAlongSpline _spline (* _index _spacing) "Local")))) (.Pitch (Math|Rotator|BreakRotator (Spline|GetRotationatDistanceAlongSpline _spline (* _index _spacing) "Local"))) (.Yaw (Math|Rotator|BreakRotator (Spline|GetRotationatDistanceAlongSpline _spline (* _index _spacing) "Local")))))))
    (Components|StaticMesh|SetStaticMesh _returnvalue "/Game/BluePrints/Chains/Chain_Link_Resized.Chain_Link_Resized")
    (Rendering|Material|SetMaterial _returnvalue 0 "/Game/BluePrints/Towers/ElixirCollector/Materials/Metal_Inst.Metal_Inst")))