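; Rear castle arena piece that takes on blue or red team colors.
; The construction script reads IsTeamBlue and swaps the shingle, dark trim and rhombus pattern materials on RearCastleResized, plus the Curtains material, to the matching team set.
; The color choice is applied at construction, and the event graph holds only disabled stub events with no runtime logic.
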(event EventBeginPlay)

(event Collision|EventActorBeginOverlap
  (params (OtherActor :type Actor%20Object%20Reference)))

(event EventTick
  (params (DeltaSeconds :type Float%20%28single-precision%29)))

(fn ConstructionScript
  (bind _curtains (Variables|Default|GetCurtains))
  (bind _rear_castle_resized (Variables|Default|GetRear_Castle_Resized))
  (if (Variables|Default|GetIsTeamBlue?)
    (Rendering|Material|SetMaterial _rear_castle_resized 0 "/Game/Materials/Instances/Shingles_Inst_Blue.Shingles_Inst_Blue")
    (Rendering|Material|SetMaterial _rear_castle_resized 1 "/Game/Materials/Instances/Basic_Colors/Dark_Blue_Inst.Dark_Blue_Inst")
    (Rendering|Material|SetMaterial _rear_castle_resized 6 "/Game/Materials/Instances/RhombusPattern_Blue_Inst.RhombusPattern_Blue_Inst")
    (Rendering|Material|SetMaterial _curtains 0 "/Game/Materials/Instances/Basic_Colors/Dark_Blue_Inst.Dark_Blue_Inst")
    (else
      (Rendering|Material|SetMaterial _rear_castle_resized 0 "/Game/Materials/Instances/Shingles_Inst_Red.Shingles_Inst_Red")
      (Rendering|Material|SetMaterial _rear_castle_resized 1 "/Game/Materials/Instances/Basic_Colors/Dark_Red_Inst.Dark_Red_Inst")
      (Rendering|Material|SetMaterial _rear_castle_resized 6 "/Game/Materials/Instances/RhombusPattern_Red_Inst.RhombusPattern_Red_Inst")
      (Rendering|Material|SetMaterial _curtains 0 "/Game/Materials/Instances/Basic_Colors/Dark_Red_Inst.Dark_Red_Inst"))))